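; BP_Statue is a collectible that jumps to random spots until the player touches it.
; InitStatue teleports it within a fixed X/Y range at zero height, then re-arms itself by timer at an interval that shortens as the game mode's Level rises.
; On player overlap, unless the game is over, it notifies BP_Guide_Gamemode, destroys itself and spawns a replacement, which relocates on BeginPlay.
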(event `self.ReceiveBeginPlay`
  (bind _asbp_guide_gamemode (cast `/Game/BP_Guide/BP_Guide_Gamemode` (`GameplayStatics.GetGameMode`)))
  (set `self.My_Guide_GameMode` _asbp_guide_gamemode)
  (`self.InitStatue`))

(event `self.ReceiveActorBeginOverlap`
  (params (OtherActor :type "Actor Object Reference"))
  (if (and (== OtherActor (`GameplayStatics.GetPlayerCharacter` 0)) (not (`/Game/BP_Guide/BP_Guide_Gamemode.GameOver` (`self.My_Guide_GameMode`))))
    (`/Game/BP_Guide/BP_Guide_Gamemode.Statue Collected` (`self.My_Guide_GameMode`))
    (`self.K2_DestroyActor`)
    (`|SpawnActorFromClass` "BP_Statue_C" (`self.GetTransform`) "Undefined" "OverrideRootScale" null null)))

(fn `InitStatue`
  (`self.K2_TeleportTo` (`KismetMathLibrary.MakeVector` (`KismetMathLibrary.RandomFloatInRange` -200.0 3000.0) (`KismetMathLibrary.RandomFloatInRange` -200.0 3000.0) 0.0))
  (`KismetSystemLibrary.K2_SetTimer` null "InitStatue" (`KismetMathLibrary.Conv_IntToDouble` (- 6 (`/Game/BP_Guide/BP_Guide_Gamemode.Level` (`self.My_Guide_GameMode`))))))

(fn `UserConstructionScript`)